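; BP_Chest is a chest actor that spawns a random item the first time it is opened.
; OpenChest checks the IsOpen flag, spawns a random class from the ClassObjectSpawn array slightly offset from its Scene component, then sets the flag so later calls spawn nothing.
; A debug print shows the flag on each call, and the event graph holds only disabled stub events, so OpenChest relies on an external caller.
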(fn `OpenChest`
  (bind _isopen (`self.IsOpen`))
  (`KismetSystemLibrary.PrintString` (`KismetStringLibrary.Conv_BoolToString` _isopen))
  (if (not _isopen)
    (`|SpawnActorFromClass` (`KismetArrayLibrary.Array_Random` (`self.ClassObjectSpawn`)) (`KismetMathLibrary.MakeTransform` (+ (`SceneComponent.K2_GetComponentLocation` (`self.Scene`)) (0.0 -40.0 0.0))) "Undefined" "OverrideRootScale" null null)
    (set `self.IsOpen` true)))

(fn `UserConstructionScript`)